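; BP_P_Knight is the player Knight Blueprint, supplying the character's attack hit check.
; AttackCollisionCheck runs a Pawn sphere overlap, offset left or right along X by orientation, with a debug sphere drawn at the same spot.
; Each overlapped actor tagged "enemy" receives a hit interface message carrying the Knight as causer, PlayerDamage and a fixed knockback force.
; BeginPlay, overlap and Tick events are unused, and construction defers to the parent.
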(event `self.Attack_Collision_Check`
  (bind _returnvalue (+ (`self.K2_GetActorLocation`) (`KismetMathLibrary.MakeVector` (select `/Game/Blueprints/E_Orientation` (`self.E_Orientation`) :`NewEnumerator0` 19.0 :`NewEnumerator1` 19.0 :`NewEnumerator2` -19.0))))
  (`KismetSystemLibrary.DrawDebugSphere` _returnvalue 20.0 12 (struct :`R` 1.0 :`G` 1.0 :`B` 1.0 :`A` 1.0) 4.0 0.6)
  (bind (_outactors _returnvalue_2) (`KismetSystemLibrary.SphereOverlapActors` _returnvalue 20.0 (`|MakeArray` "ObjectTypeQuery3" :!type "EObjectTypeQuery Enum") null (`|MakeArray` self :!type "Actor Object Reference")))
  (if _returnvalue_2
    (for _array_element _outactors
      (if (`self.ActorHasTag` _array_element "enemy")
        (message `/Game/Blueprints/Interfaces/BPI_Combat.BPI_HitHandle` _array_element self (`self.PlayerDamage`) 300)))))

(fn `UserConstructionScript`
  (`parent.UserConstructionScript`))