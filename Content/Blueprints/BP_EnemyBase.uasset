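; BP_EnemyBase is an enemy base Blueprint that, so far, only reacts to hit messages with a debug readout.
; Its BPIHitHandle event, apparently from a hit interface, prints the causer's name, damage and knockback force on screen for an extended duration.
; No damage or knockback is applied, the default events are disabled stubs, and the construction script only calls its parent.
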(event `/Game/Blueprints/Interfaces/BPI_Combat.BPI_HitHandle`
  (params (Causer :type "Actor Object Reference") (Damage :type "Float (double-precision)") (KnockBackForce :type Integer))
  (`KismetSystemLibrary.PrintString` (`KismetStringLibrary.Concat_StrStr` (`KismetSystemLibrary.GetDisplayName` Causer) " | " (`KismetStringLibrary.Conv_DoubleToString` Damage) " | " (`KismetStringLibrary.Conv_IntToString` KnockBackForce)) true true (struct :`G` 0.66 :`B` 1.0 :`A` 1.0) 30.0))

(fn `UserConstructionScript`
  (`parent.UserConstructionScript`))