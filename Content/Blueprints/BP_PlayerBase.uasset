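; Base player character for a networked side-scroller, handling move, jump, roll and attack through Enhanced Input and state-check gates.
; Server events set facing, roll and attack state, then multicast override animations on the AnimationComponent.
; Rolling lerps the actor along its facing via timeline, stopping when a line trace hits static obstacles.
; Attack collision is an empty hook, and an interface event replicates movement locking by multicast.
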(event `EnhancedInput|/Game/Input/IA_Jump`
  (params (ActionValue :type Boolean) (ElapsedSeconds :type "Float (double-precision)") (TriggeredSeconds :type "Float (double-precision)") (InputAction :type "InputAction Object Reference" :default "/Game/Input/IA_Jump.IA_Jump"))
  (:`Started`
    (`self.CanDoJump`)
    (`self.Jump`))
  (:`Canceled`
    (`self.StopJumping` :!label _label))
  (:`Completed`
    (goto _label)))

(event `EnhancedInput|/Game/Input/IA_Move`
  (params (ActionValue :type "Float (double-precision)") (ElapsedSeconds :type "Float (double-precision)") (TriggeredSeconds :type "Float (double-precision)") (InputAction :type "InputAction Object Reference" :default "/Game/Input/IA_Move.IA_Move"))
  (:`Triggered`
    (`self.CanMove`)
    (`self.AddMovementInput` (`KismetMathLibrary.GetForwardVector` (`self.GetControlRotation`)) ActionValue)
    (if (!= ActionValue 0.0)
      (if (> ActionValue 0.0)
        (`self.Server_ChangeOrientation` "NewEnumerator1")
        (else
          (`self.Server_ChangeOrientation` "NewEnumerator2"))))))

(event `Server_ChangeOrientation`
  (params (Orientation :type "/Game/Blueprints/E_Orientation Enum" :default "NewEnumerator0"))
  (set `self.E_Orientation` Orientation))

(event `EnhancedInput|/Game/Input/IA_Roll`
  (params (ActionValue :type Boolean) (ElapsedSeconds :type "Float (double-precision)") (TriggeredSeconds :type "Float (double-precision)") (InputAction :type "InputAction Object Reference" :default "/Game/Input/IA_Roll.IA_Roll"))
  (:`Triggered`
    (`self.CanRoll`)
    (`self.Server_Rolling`)))

(event `Server_Rolling`
  (`self.CanRoll`)
  (set `self.IsRolling` true)
  (`self.CheckRollingTargetLocation`)
  (`self.Multicast_Anim` (`self.RollingAnim`))
  (bind (_direction _alpha) (`Timeline|TL_Rolling` :!via `PlayFromStart`)
    (:`Update`
      (`self.K2_SetActorLocation` (`KismetMathLibrary.VLerp` (`self.K2_GetActorLocation`) (`self.RollingTargetLocation`) _alpha))
      (`self.CheckObstacles`))))

(event `Multicast_Anim`
  (params (AnimSequence :type "PaperZDAnimSequence Object Reference"))
  (`PaperZDPlaySlotOverrideAction.PlayAnimationOverrideWithCallbacks` (`PaperZDAnimationComponent.AnimInstance` (`self.AnimationComponent`)) AnimSequence "MyAnimSlot"))

(event `EnhancedInput|/Game/Input/IA_Atk`
  (params (ActionValue :type Boolean) (ElapsedSeconds :type "Float (double-precision)") (TriggeredSeconds :type "Float (double-precision)") (InputAction :type "InputAction Object Reference" :default "/Game/Input/IA_Atk.IA_Atk"))
  (:`Triggered`
    (`self.CanAtk`)
    (`self.Server_Attack`)))

(event `Server_Attack`
  (`self.CanAtk`)
  (set `self.IsAttacking` true)
  (`|ExecutionSequence`
    (:`then_0`
      (`self.Multicast_Anim` (`self.AtkAnim`))
      (`KismetSystemLibrary.Delay` 0.8)
      (set `self.AllowMoving` true)
      (set `self.IsAttacking` false))
    (:`then_1`
      (`self.Attack_Collision_Check`))))

(event `Attack_Collision_Check`)

(event `/Game/Blueprints/Interfaces/BPI_Combat.BPI_NotMoving`
  (params (AllowMoving :type Boolean))
  (`self.Server_NotMoving` AllowMoving))

(event `Server_NotMoving`
  (params (AllowMoving :type Boolean))
  (`self.Multicast_NotMoving` AllowMoving))

(event `Multicast_NotMoving`
  (params (AllowMoving :type Boolean))
  (set `self.AllowMoving` AllowMoving))

(fn `CheckObstacles`
  (bind _returnvalue (`self.K2_GetActorLocation`))
  (bind (_outhit _returnvalue_2) (`KismetSystemLibrary.LineTraceSingleForObjects` :`Start` _returnvalue :`End` (+ _returnvalue (* (`self.GetActorForwardVector`) (select `/Game/Blueprints/E_Orientation` (`self.E_Orientation`) :`NewEnumerator0` 50 :`NewEnumerator1` 50 :`NewEnumerator2` -50))) :`ObjectTypes` (`|MakeArray` "ObjectTypeQuery1" :!type "EObjectTypeQuery Enum") :`DrawDebugType` "ForDuration"))
  (if _returnvalue_2
    (`TimelineComponent.Stop` (`self.TL_Rolling`))))

(fn `CheckRollingTargetLocation`
  (set `self.RollingTargetLocation` (+ (`self.K2_GetActorLocation`) (* (`self.GetActorForwardVector`) (select `/Game/Blueprints/E_Orientation` (`self.E_Orientation`) :`NewEnumerator0` 200 :`NewEnumerator1` 200 :`NewEnumerator2` -200)))))

(fn `UserConstructionScript`
  (`parent.UserConstructionScript`))