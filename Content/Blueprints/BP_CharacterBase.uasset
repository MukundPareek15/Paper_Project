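; Base character Blueprint with a Sprite component, providing networked facing and floating damage numbers.
; A RepNotify on the orientation enum rotates the sprite to face right or left.
; A server event spawns a damage text actor just above the passed-in Instigator, which it stores as the damage target, then multicasts the number in white.
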(event `Server_SpawnDamageTextActor`
  (params (Instigator :type "Actor Object Reference") (DamageNumber :type "Float (double-precision)"))
  (bind _output_get (set `self.DamageTarget` Instigator))
  (bind (_returnvalue_x _returnvalue_y _returnvalue_z) (`KismetMathLibrary.BreakVector` (`self.K2_GetActorLocation` _output_get)))
  (bind _returnvalue (`|SpawnActorFromClass` "/Game/Blueprints/BPA/BPA_Damage_Text.BPA_Damage_Text_C" (`KismetMathLibrary.MakeTransform` (`KismetMathLibrary.MakeVector` _returnvalue_x _returnvalue_y (+ _returnvalue_z 2.0))) "Undefined" "MultiplyWithRoot" null null))
  (`/Game/Blueprints/BPA/BPA_Damage_Text.Multicast_UpdateDmgNumber` _returnvalue DamageNumber (struct :`R` 1.0 :`G` 1.0 :`B` 1.0 :`A` 1.0)))

(fn `OnRep_E_Orientation`
  (bind _sprite (`self.Sprite`))
  (switch `/Game/Blueprints/E_Orientation` (`self.E_Orientation`)
    (:`NewEnumerator1`
      (`SceneComponent.K2_SetRelativeRotation` :`self` _sprite))
    (:`NewEnumerator2`
      (`SceneComponent.K2_SetRelativeRotation` _sprite (struct :`Yaw` 180.0) false false))))

(fn `UserConstructionScript`)